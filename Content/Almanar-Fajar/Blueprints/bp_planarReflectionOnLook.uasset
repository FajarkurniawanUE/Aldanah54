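; Planar reflection Blueprint that shows its reflection only while its linked MirrorActor is on screen, starting hidden.
; Each tick it checks whether the mirror was recently rendered and toggles the PlanarReflectionComponent's visibility.
; A pair of cross-reset DoOnce gates limits the show and hide calls to changes in that state.
; While the player pawn is a pawn_dollhouse, the reflection is forced hidden every tick.
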(event EventTick
  (params (DeltaSeconds :type Float%20%28single-precision%29))
  (bind _planarreflectioncomponent (Variables|Default|GetPlanarReflectionComponent))
  (Utilities|Casting|CastTopawn_dollhouse (Game|Player|GetPlayerPawn 0)
    (:then
      (Rendering|SetVisibility (Variables|Default|GetPlanarReflectionComponent) false false))
    (:CastFailed
      (if (Class|Actor|WasRecentlyRendered (Variables|Default|GetMirrorActor) 0.2)
        (Utilities|FlowControl|Sequence
          (:then_0
            (Utilities|FlowControl|DoOnce false :!label _label
              (:Completed
                (Rendering|SetVisibility _planarreflectioncomponent true false))))
          (:then_1
            (goto _label_2 Reset)))
        (else
          (Utilities|FlowControl|Sequence
            (:then_0
              (goto _label Reset))
            (:then_1
              (Utilities|FlowControl|DoOnce false :!label _label_2
                (:Completed
                  (Rendering|SetVisibility _planarreflectioncomponent false false))))))))))

(event EventBeginPlay
  (Rendering|SetVisibility (Variables|Default|GetPlanarReflectionComponent) false false))

(fn ConstructionScript)