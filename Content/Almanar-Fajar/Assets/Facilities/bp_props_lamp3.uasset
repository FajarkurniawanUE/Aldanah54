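; Lamp prop Blueprint for the facilities set, with a spot light that can be switched on or off.
; The construction script sets the spot light's visibility from the Light variable and, when lit, applies the CastShadow setting.
; The props_lamp event repeats the same toggle at runtime from a Condition input, propagating visibility to child components.
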(event Custom|props_lamp
  (params (Condition :type Boolean))
  (bind _spotlight (Variables|Default|GetSpotLight))
  (if Condition
    (Rendering|SetVisibility _spotlight true true)
    (Rendering|Components|Light|SetCastShadows _spotlight (Variables|Default|GetCast%20Shadow))
    (else
      (Rendering|SetVisibility _spotlight false true))))

(fn ConstructionScript
  (bind _spotlight (Variables|Default|GetSpotLight))
  (if (Variables|Default|GetLight)
    (Rendering|SetVisibility _spotlight true true)
    (Rendering|Components|Light|SetCastShadows _spotlight (Variables|Default|GetCast%20Shadow))
    (else
      (Rendering|SetVisibility _spotlight false true))))