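; BP_array_generator is a construction-script tool that lays out a grid of house mesh instances.
; It sets SMHouse on a Hierarchical Instanced Static Mesh, then nested loops add instances by row count, per-row count and spacing, with rows stepping along negative X.
; Toggles pick random quarter-turn yaw or a 180-degree flip on alternate rows, and random uniform or unit scale.
; Randomness is unseeded, and the event graph is unused.
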(event EventBeginPlay)

(event Collision|EventActorBeginOverlap
  (params (OtherActor :type Actor%20Object%20Reference)))

(event EventTick
  (params (DeltaSeconds :type Float%20%28single-precision%29)))

(fn ConstructionScript
  (Components|StaticMesh|SetStaticMesh (Variables|Default|GetHierarchicalInstancedStaticMesh) (Variables|Default|GetSM_House))
  (for _index (range 0 (- (Variables|Default|GetNumberOfRows) 1))
    (Variables|Default|SetInstanceLocationX (- 1.0 (* _index (Variables|Default|GetSpaceBetweenRows))))
    (for _index_2 (range 0 (- (Variables|Default|GetInstancesPerRow) 1))
      (Components|InstancedStaticMesh|AddInstance (Variables|Default|GetHierarchicalInstancedStaticMesh) (Math|Transform|MakeTransform (Math|Vector|MakeVector (Variables|Default|GetInstanceLocationX) (* _index_2 (Variables|Default|GetSpaceBetweenInstances)) 0.0) (Math|Rotator|MakeRotator 0.0 0.0 (Math|Float|SelectFloat (Utilities|Select :Index (Math|Random|RandomIntegerinRange 0 3) :Option%200 0.0 :Option%201 9e+01 :Option%202 1.8e+02 :Option%203 2.7e+02) (Math|Conversions|ToFloat(Integer) (* _index 180)) (Variables|Default|GetRandomRotation))) (Math|Vector|SelectVector (Math|Conversions|ToVector(Float) (Math|Random|RandomFloatinRange (Variables|Default|GetMin%20Scale) (Variables|Default|GetMax%20Scale))) "1.000000,1.000000,1.000000" (Variables|Default|GetRandomScale))) false))))