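; Base house actor that shows unit info and lets the player enter houses that have interiors.
; On Tick, a match between char_roshn_exterior's traced component and its Box toggles the info widget and input, so Enter or gamepad top button calls the widget's GoToLevel.
; For other pawns it fills the go-inside VR widget and disables Box collision.
; The construction script mirrors via negative Y scale and toggles plant and wall-light visibility and mobility.
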(event Custom|beingTrace
  (bind _widget (Variables|Default|GetWidget))
  (Input|EnableInput (Game|GetPlayerController 0))
  (Utilities|FlowControl|Sequence
    (:then_0
      (Utilities|FlowControl|DoOnce false
        (:Completed
          (Rendering|SetVisibility _widget true false))))
    (:then_1
      (Utilities|FlowControl|DoOnce false) ; enters at Reset
    )))

(event Custom|notTrace
  (bind _widget (Variables|Default|GetWidget))
  (Input|DisableInput (Game|GetPlayerController 0))
  (Utilities|FlowControl|Sequence
    (:then_0
      (Utilities|FlowControl|DoOnce false) ; enters at Reset
    )
    (:then_1
      (Utilities|FlowControl|DoOnce false
        (:Completed
          (Rendering|SetVisibility _widget false false))))))

(event EventBeginPlay
  (Rendering|SetVisibility (Variables|Default|GetWidgetgoinside) true false)
  (bind _aschar_roshn_exterior (Utilities|Casting|CastTochar_roshn_exterior (Game|GetPlayerCharacter 0))
    (:then
      (Variables|Default|SetAs%20Char%20Roshn%20Exterior _aschar_roshn_exterior)
      (bind _asumg_unit_info (Utilities|Casting|CastToumg_unit_info (UserInterface|GetUserWidgetObject (Variables|Default|GetWidget))))
      (Variables|/Game/FajarRoshn/UMG/umg_unit_info.umg_unit_info_C|SetUnit%20Type_0 _asumg_unit_info (Variables|Default|GetUnit%20Type))
      (if (Variables|Default|GetHas%20Interior)
        (Default|ShowEnter _asumg_unit_info)))
    (:CastFailed
      (bind _asumg_goinside_vr_1 (Utilities|Casting|CastToumg_goinside_vr1 (UserInterface|GetUserWidgetObject (Variables|Default|GetWidgetgoinside))))
      (Variables|/Game/FajarRoshn/UMG/umg_goinside_vr1.umg_goinside_vr1_C|Setunit%20name _asumg_goinside_vr_1 (Variables|Default|GetUnit%20name))
      (Variables|/Game/FajarRoshn/UMG/umg_goinside_vr1.umg_goinside_vr1_C|SetUnit%20Type_0 _asumg_goinside_vr_1 (Variables|Default|GetUnit%20Type))
      (Variables|/Game/FajarRoshn/UMG/umg_goinside_vr1.umg_goinside_vr1_C|Setstyle _asumg_goinside_vr_1 (Variables|Default|GetStyle))
      (Collision|SetCollisionEnabled (Variables|Default|GetBox) "NoCollision"))))

(event EventTick
  (params (DeltaSeconds :type Float%20%28single-precision%29))
  (bind _as_char_roshn_exterior (Variables|Default|GetAs%20Char%20Roshn%20Exterior))
  (if (Variables|Default|GetTracable)
    (Utilities|IsValid _as_char_roshn_exterior
      (:Is%20Valid
        (if (== (Variables|/Game/FajarRoshn/Blueprints/char_roshn_exterior.char_roshn_exterior_C|GetcurrentTracingComponent _as_char_roshn_exterior) (Variables|Default|GetBox))
          (CallFunction|BeingTrace)
          (else
            (CallFunction|NotTrace)))))))

(event Input|KeyboardEvents|Enter
  (params (Key :type Key%20Structure :default "None"))
  (:Released
    (if (Variables|Default|GetHas%20Interior)
      (bind _asumg_unit_info (Utilities|Casting|CastToumg_unit_info (UserInterface|GetUserWidgetObject (Variables|Default|GetWidget))))
      (Default|GotoLevel _asumg_unit_info))))

(event Input|GamepadEvents|GamepadFaceButtonTop
  (params (Key :type Key%20Structure :default "None"))
  (:Released
    (if (Variables|Default|GetHas%20Interior)
      (bind _asumg_unit_info (Utilities|Casting|CastToumg_unit_info (UserInterface|GetUserWidgetObject (Variables|Default|GetWidget))))
      (Default|GotoLevel _asumg_unit_info))))

(fn ConstructionScript
  (Transformation|SetRelativeScale3D (Variables|Default|GetDefaultSceneRoot) (Math|Vector|SelectVector "1.000000,-1.000000,1.000000" "1.000000,1.000000,1.000000" (Variables|Default|GetMirror)))
  (Transformation|SetRelativeScale3D (Variables|Default|GetWidgetgoinside) (Math|Vector|SelectVector "0.600000,-0.600000,0.600000" "0.600000,0.600000,0.600000" (Variables|Default|GetMirror)))
  (for _array_element (Components|GetChildrenComponents (Variables|Default|GetPlants) true)
    (Transformation|SetMobility _array_element (select (Variables|Default|GetUse%20Plants) "Static" "Movable"))
    (Rendering|SetVisibility _array_element (Variables|Default|GetUse%20Plants) true)
    (for _array_element_2 (Components|GetChildrenComponents (Variables|Default|GetDefaultSceneRoot) true)
      (bind _aslight_spotwall (Utilities|Casting|CastTolight_spotwall _array_element_2))
      (Rendering|SetVisibility _aslight_spotwall (Variables|Default|GetUse%20Lights) false)
      (Transformation|SetMobility _aslight_spotwall (select (Variables|Default|GetUse%20Lights) "Static" "Movable")))))