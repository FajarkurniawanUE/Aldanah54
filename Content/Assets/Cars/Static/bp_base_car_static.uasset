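; Base Blueprint for a static car prop with a configurable mesh and a randomized paint color.
; The construction script assigns the Car mesh to the SmCar component and creates a dynamic material instance from its first material slot.
; It sets that instance's Color parameter to a random entry from the Colors array, while the event graph holds no active logic.
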(event EventBeginPlay)

(event Collision|EventActorBeginOverlap
  (params (OtherActor :type Actor%20Object%20Reference)))

(event EventTick
  (params (DeltaSeconds :type Float%20%28single-precision%29)))

(fn ConstructionScript
  (bind _sm_car (Variables|Default|Getsm_car))
  (Components|StaticMesh|SetStaticMesh (Variables|Default|Getsm_car) (Variables|Default|GetCar))
  (bind _returnvalue (Rendering|Material|CreateDynamicMaterialInstance _sm_car 0 (Rendering|Material|GetMaterial _sm_car 0) "None" :!class /Script/Engine.PrimitiveComponent))
  (Rendering|Material|SetVectorParameterValue _returnvalue "Color" (.OutItem (Utilities|Array|Random (Variables|Default|GetColors))) :!class /Script/Engine.MaterialInstanceDynamic)
  (Rendering|Material|SetMaterial (Variables|Default|Getsm_car) 0 _returnvalue))